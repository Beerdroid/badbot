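; Player-controlled flying bot pawn that shoots blaster beams, adds the overlay HUD and quits the game when its health runs out.
; Enhanced Input drives look and three-axis movement relative to control rotation through FloatingPawnMovement.
; Each shot alternates between left and right rifle sockets via FlipFlop, spawning a beam actor with burst FX and sound.
; A camera-forward line trace sets the aim point, so beams from either socket converge on the view target.
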(event Input|EnhancedActionEvents|EnhancedInputActionIA_Fire
  (params (ActionValue :type Boolean) (ElapsedSeconds :type Float%20%28double-precision%29) (TriggeredSeconds :type Float%20%28double-precision%29) (InputAction :type Input%20Action%20Object%20Reference :default "/Game/Blueprints/Input/InputActions/IA_Fire.IA_Fire"))
  (:Started
    (Utilities|FlowControl|FlipFlop
      (:A
        (CallFunction|SpawnBlasterBeam "Rifle_L"))
      (:B
        (CallFunction|SpawnBlasterBeam "Rifle_R")))))

(event Input|EnhancedActionEvents|EnhancedInputActionIA_Look
  (params (ActionValue :type Vector%202D%20Structure) (ElapsedSeconds :type Float%20%28double-precision%29) (TriggeredSeconds :type Float%20%28double-precision%29) (InputAction :type Input%20Action%20Object%20Reference :default "/Game/Blueprints/Input/InputActions/IA_Look.IA_Look"))
  (bind (_x _y) (Math|Vector2D|BreakVector2D ActionValue))
  (Pawn|Input|AddControllerYawInput _x)
  (Pawn|Input|AddControllerPitchInput _y))

(event Input|EnhancedActionEvents|EnhancedInputActionIA_Move
  (params (ActionValue :type Vector :default "0, 0, 0") (ElapsedSeconds :type Float%20%28double-precision%29) (TriggeredSeconds :type Float%20%28double-precision%29) (InputAction :type Input%20Action%20Object%20Reference :default "/Game/Blueprints/Input/InputActions/IA_Move.IA_Move"))
  (Class|PawnMovementComponent|AddInputVector (Variables|Default|GetFloatingPawnMovement) (* (Math|Vector|GetRightVector (Pawn|GetControlRotation :!class /Script/Engine.Pawn)) (.x (Input|EnhancedActionValues|GetIA_Move))) false)
  (Class|PawnMovementComponent|AddInputVector (Variables|Default|GetFloatingPawnMovement) (* (Math|Vector|GetForwardVector (Pawn|GetControlRotation :!class /Script/Engine.Pawn)) (.y (Input|EnhancedActionValues|GetIA_Move))) false)
  (Class|PawnMovementComponent|AddInputVector (Variables|Default|GetFloatingPawnMovement) (* (Math|Vector|GetUpVector (Pawn|GetControlRotation :!class /Script/Engine.Pawn)) (.z (Input|EnhancedActionValues|GetIA_Move))) false))

(event EventBeginPlay
  (Utilities|FlowControl|Sequence
    (:then_0
      (bind _returnvalue (UserInterface|CreateWidget "/Game/Blueprints/UI/WBP_OverlayHUD.WBP_OverlayHUD_C"))
      (UserInterface|Viewport|AddtoViewport _returnvalue 0))
    (:then_1
      (bind _asplayer_controller (Utilities|Casting|CastToPlayerController (Pawn|GetController)))
      (Input|AddMappingContext (PlayerController|LocalPlayerSubsystems|GetEnhancedInputLocalPlayerSubsystem _asplayer_controller) "/Game/Blueprints/Input/IMC_Bot.IMC_Bot" 0 "(bIgnoreAllPressedKeysUntilRelease=True,bForceImmediately=False,bNotifyUserSettings=False)"))))

(event EventGetHurt
  (params (Damage :type Float%20%28double-precision%29))
  (bind _output_get (Variables|Default|SetHealth (- (Variables|Default|GetHealth) Damage)))
  (Development|PrintString (Utilities|String|ToString(Float) _output_get))
  (if (<= (Variables|Default|GetHealth) 0.0)
    (Game|QuitGame 0 "Quit" false)))

(fn ConstructionScript)

(fn SpawnBlasterBeam
  (params (SocketName :type Name))
  (bind _staticmesh (Variables|Default|GetStaticMesh))
  (bind _returnvalue (Transformation|GetSocketTransform _staticmesh SocketName "RTS_World"))
  (LocalVariables|SetTraceEnd (CallFunction|GetTraceEnd))
  (bind _outhit (Collision|LineTraceByChannel (Transformation|GetWorldLocation (Variables|Default|GetCamera)) (LocalVariables|GetTraceEnd) "TraceTypeQuery1" false 0 "None"))
  (LocalVariables|SetTraceEnd (Math|Vector|SelectVector (.ImpactPoint (Collision|BreakHitResult _outhit)) (LocalVariables|GetTraceEnd) (.bBlockingHit (Collision|BreakHitResult _outhit))))
  (Game|SpawnActorfromClass "/Game/Blueprints/BlasterBEam/BP_PlayerBlasterBeam.BP_PlayerBlasterBeam_C" (Math|Transform|MakeTransform (.location _returnvalue) (Math|Rotator|FindLookatRotation (.location _returnvalue) (LocalVariables|GetTraceEnd)) "1.000000,1.000000,1.000000") "Undefined" "MultiplyWithRoot" 0 0 0)
  (CallFunction|SpawnFireFX SocketName))

(fn GetTraceEnd
  (bind _camera (Variables|Default|GetCamera))
  (return (+ (Transformation|GetWorldLocation _camera) (* (Math|Vector|GetForwardVector _camera) (Variables|Default|GetTraceDistance)))))

(fn SpawnFireFX
  (params (SocketName :type Name))
  (bind _staticmesh (Variables|Default|GetStaticMesh))
  (bind _returnvalue (Transformation|GetSocketTransform _staticmesh SocketName "RTS_World"))
  (Niagara|SpawnSystematLocation "/Game/Assets/FX/NS_BeamBurst.NS_BeamBurst" (.location _returnvalue) (.rotation _returnvalue))
  (Audio|PlaySoundatLocation "/Game/Assets/Sounds/Sounds/Drone/sfx_EnergyRifle.sfx_EnergyRifle" (.location _returnvalue) "0, 0, 0" 0.5 1.0 0.0 0 0 0 0))