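; BP_SmallSphere is a short-lived moving pickup that increments the BP_BadBotGameMode score when a BP_BotPawn overlaps it.
; Each tick it advances along its forward vector and applies a scaled random spin chosen at spawn, so its heading keeps changing.
; Timelines scale the mesh on spawn and on wink-out, which is triggered by overlap or lifetime expiry, guarded against replay, and ends in destruction.
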(event Custom|WinkOut
  ;[0.9062 0.105 0.057 0.5] Wink Out
  (if (not (Variables|Default|GetIsWinking))
    (Variables|Default|SetIsWinking true)
    (bind _scale (Timeline|WinkOutTimeline Play)
      (:Update
        (CallFunction|ScaleSphere _scale))
      (:Finished
        (Actor|DestroyActor)))))

(event Custom|WinkIn
  (bind _scale (Timeline|WinkInTimeline Play)
    (:Update
      (Transformation|SetWorldScale3D (Variables|Default|GetStaticMesh) _scale))))

(event Custom|OnSphereOverlap
  (params (OverlappedComponent :type Primitive%20Component%20Object%20Reference) (OtherActor :type Actor%20Object%20Reference) (OtherComp :type Primitive%20Component%20Object%20Reference) (OtherBodyIndex :type Integer) (bFromSweep :type Boolean) (SweepResult :type Hit%20Result%20Structure%20%28by%20ref%29))
  ;[0.04862 0.15 0.03155 0.5] HandleOverlap
  (if (Class|GameplayStatics|ObjectIsA OtherActor "/Game/Blueprints/BotPawn/BP_BotPawn.BP_BotPawn_C")
    (bind _asbp_bad_bot_game_mode (Utilities|Casting|CastToBP_BadBotGameMode (Game|GetGameMode)))
    (Default|IncrementScore _asbp_bad_bot_game_mode)
    (CallFunction|WinkOut)))

(event EventBeginPlay
  (CallFunction|Winkin)
  (CallFunction|InitializeDeltaRotation)
  ;[0.9062 0.105 0.057 0.5] Wink Out
  (Utilities|Time|SetTimerbyEvent (delegate Custom|WinkOut) (Variables|Default|GetLifeTime))
  ;[0.04862 0.15 0.03155 0.5] HandleOverlap
  (Collision|AssignOnComponentBeginOverlap (Variables|Default|GetSphereVolume) (delegate Custom|OnSphereOverlap)))

(event EventTick
  (params (DeltaSeconds :type Float%20%28single-precision%29))
  (CallFunction|UpdateLocation DeltaSeconds)
  (CallFunction|UpdateRotation DeltaSeconds))

(fn ConstructionScript)

(fn InitializeDeltaRotation
  (Variables|Default|SetDeltaRotation (* (Math|Random|RandomRotator false) (Variables|Default|GetRotationScaleFactor))))

(fn UpdateLocation
  (params (DeltaSeconds :type Float%20%28double-precision%29))
  (Transformation|AddActorWorldOffset (* (Transformation|GetActorForwardVector) (* DeltaSeconds (Variables|Default|GetSpeed)))))

(fn UpdateRotation
  (params (DeltaSeconds :type Float%20%28single-precision%29))
  (Transformation|AddActorLocalRotation (* (Variables|Default|GetDeltaRotation) DeltaSeconds) false false))

(fn ScaleSphere
  (params (InputPin :type Float%20%28single-precision%29))
  (Transformation|SetWorldScale3D (Variables|Default|GetStaticMesh) (Math|Vector|MakeVector InputPin InputPin InputPin)))